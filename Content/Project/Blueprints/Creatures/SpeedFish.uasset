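; SpeedFish is a playable fish creature whose ability is a swim speed boost.
; Holding IA_Ability raises the CharacterMovement max swim speed and sets IsSwimmingFast; completing or canceling it restores the slower speed.
; Each Tick updates speed particles and, while boosted with movement input, plays the Getaway timeline to widen the follow camera's field of view, otherwise reversing it.
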(event `EnhancedInput|/Game/ThirdPerson/Input/Actions/IA_Ability`
  (params (ActionValue :type Boolean) (ElapsedSeconds :type "Float (double-precision)") (TriggeredSeconds :type "Float (double-precision)") (InputAction :type "InputAction Object Reference" :default "/Game/ThirdPerson/Input/Actions/IA_Ability.IA_Ability"))
  (bind _charactermovement (`self.CharacterMovement`))
  (:`Triggered`
    (set `CharacterMovementComponent.MaxSwimSpeed` 1900.0 _charactermovement :!label _label)
    (set `self.isSwimmingFast` true))
  (:`Started`
    (goto _label))
  (:`Canceled`
    (set `CharacterMovementComponent.MaxSwimSpeed` 1300.0 _charactermovement :!label _label_2)
    (set `self.isSwimmingFast` false))
  (:`Completed`
    (goto _label_2)))

(event `self.ReceiveTick`
  (params (DeltaSeconds :type "Float (single-precision)"))
  (`self.CalculateSpeedParticles`)
  (if (and (not (`KismetMathLibrary.IsZero2D` (`|GetInputActionValue`))) (`self.isSwimmingFast`))
    (bind (_direction _newtrack_1) (`Timeline|getaway` :!label _label_3)
      (:`Update`
        (`CameraComponent.SetFieldOfView` (`self.FollowCamera`) (`KismetMathLibrary.Lerp` 90.0 120.0 _newtrack_1))))
    (else
      (goto _label_3 :!via `Reverse`))))

(fn `UserConstructionScript`
  (`parent.UserConstructionScript`))