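; Door2 is a double door actor that opens on request and also serves as the game's exit point.
; An Open event runs once, guarded by a flag, and plays a timeline that yaws the two door pivots.
; When a PlayableCharacter overlaps the actor, a second timeline darkens the screen through the Proto3GameMode player UI, then quits the game when finished.
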(event `self.ReceiveActorBeginOverlap`
  (params (OtherActor :type "Actor Object Reference"))
  (cast `/Game/Project/Blueprints/Character/PlayableCharacter` OtherActor)
  (bind (_direction _newtrack_0) (`Timeline|Timeline_0` :!via `PlayFromStart`)
    (:`Update`
      (bind _asproto_3game_mode (cast `/Game/Project/Blueprints/Character/Proto3GameMode` (`GameplayStatics.GetGameMode`)))
      (`/Game/Project/Blueprints/UI/PlayerUI.DarkenScreen` (`/Game/Project/Blueprints/Character/Proto3GameMode.PlayerUI` _asproto_3game_mode) _newtrack_0))
    (:`Finished`
      (`KismetSystemLibrary.QuitGame` null "Quit"))))

(event `Open`
  (`KismetSystemLibrary.PrintString` "Ready toopen")
  (if (not (`self.HasBeenOpened`))
    (set `self.HasBeenOpened` true)
    (`KismetSystemLibrary.PrintString` "OpeningDoor")
    (bind (_direction _door1rotation _door2rotation) (`Timeline|Timeline` :`NewTime` 1.0)
      (:`Update`
        (`SceneComponent.K2_SetRelativeRotation` (`self.Door1Pivot`) (`KismetMathLibrary.MakeRotator` 0.0 0.0 _door1rotation) false false)
        (`SceneComponent.K2_SetRelativeRotation` (`self.Door2Pivot`) (`KismetMathLibrary.MakeRotator` 0.0 0.0 _door2rotation) false false)))))

(fn `UserConstructionScript`)