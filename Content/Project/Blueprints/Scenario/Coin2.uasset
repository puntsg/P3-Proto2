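; Coin2 is a collectible coin pickup that updates the coin count in Proto3GameMode when a Character overlaps it.
; On pickup it plays a 2D jingle, hides its components and disables collision, then destroys itself once the audio finishes.
; Each tick it animates by spinning two fish meshes in pitch and a torus in yaw at RotationSpeed.
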(event `self.ReceiveActorBeginOverlap`
  (params (OtherActor :type "Actor Object Reference"))
  (cast `Character` OtherActor)
  (bind _asproto_3game_mode (cast `/Game/Project/Blueprints/Character/Proto3GameMode` (`GameplayStatics.GetGameMode`)))
  (`/Game/Project/Blueprints/Character/Proto3GameMode.UpdateCoin` _asproto_3game_mode)
  (bind _returnvalue (`GameplayStatics.SpawnSound2D` "/Game/Project/Assets/Sounds/Jak_and_Daxter_OST_-_79_-_A_Power_Cell.Jak_and_Daxter_OST_-_79_-_A_Power_Cell" 1.0 1.0 0.0 null))
  (`SceneComponent.SetVisibility` (`self.DefaultSceneRoot`) false true)
  (`self.SetActorEnableCollision` false)
  (add `AudioComponent.OnAudioFinished` _returnvalue (delegate `OnAudioFinished_Event`)))

(event `OnAudioFinished_Event`
  (`self.K2_DestroyActor`))

(event `self.ReceiveTick`
  (params (DeltaSeconds :type "Float (single-precision)"))
  (bind _returnvalue (* DeltaSeconds (`self.RotationSpeed`)))
  (`SceneComponent.K2_AddLocalRotation` (`self.Fish1`) (`KismetMathLibrary.MakeRotator` 0.0 _returnvalue) false false)
  (`SceneComponent.K2_AddLocalRotation` (`self.Fish2`) (`KismetMathLibrary.MakeRotator` 0.0 _returnvalue) false false)
  (`SceneComponent.K2_AddLocalRotation` (`self.Torus`) (`KismetMathLibrary.MakeRotator` 0.0 0.0 _returnvalue) false false))

(fn `UserConstructionScript`)