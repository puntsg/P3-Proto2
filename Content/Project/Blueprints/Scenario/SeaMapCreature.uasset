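; Sea map creature that loops along a spline route and reacts when Taki comes near.
; Tick accelerates or brakes it based on player proximity, toggling Niagara particles at a speed threshold.
; Sphere overlap registers it as Taki's current map creature, toggles the ability UI and overlay outline, and triggers a tutorial.
; Timelines blend its mesh into player tracking and back to rest; PlaySound blocks overlapping playback.
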(event `self.ReceiveBeginPlay`
  (bind _returnvalue (`KismetMaterialLibrary.CreateDynamicMaterialInstance` "/Game/Project/Materials/Outliner/Outliner.Outliner"))
  (bind _output_get (set `self.OutlineMaterialInstance` _returnvalue))
  (`MeshComponent.SetOverlayMaterial` (`self.SkeletalMesh`) _output_get))

(event `PlaySound`
  (if (not (`self.IsPlayingSound`))
    (set `self.IsPlayingSound` true)
    (bind _returnvalue (`GameplayStatics.SpawnSoundAtLocation` (`self.Sound`) (`self.K2_GetActorLocation`) (struct) 1.0 1.0 0.0 null null))
    (add `AudioComponent.OnAudioFinished` _returnvalue (delegate `OnAudioFinished_Event`))))

(event `OnAudioFinished_Event`
  (set `self.IsPlayingSound` false))

(event `self.Sphere.OnComponentBeginOverlap`
  (params (OverlappedComponent :type "PrimitiveComponent Object Reference") (OtherActor :type "Actor Object Reference") (OtherComp :type "PrimitiveComponent Object Reference") (OtherBodyIndex :type Integer) (bFromSweep :type Boolean) (SweepResult :type "HitResult Structure (by ref)"))
  (bind _skeletalmesh (`self.SkeletalMesh`))
  (bind _astaki (cast `/Game/Project/Blueprints/Character/Taki` OtherActor))
  (`/Game/Project/Blueprints/Character/PlayableCharacter.SetUIAbilityState` _astaki true)
  (set `/Game/Project/Blueprints/Character/Taki.CurrentPoiningMapCreature` self _astaki)
  (bind _asproto_3game_mode (cast `/Game/Project/Blueprints/Character/Proto3GameMode` (`GameplayStatics.GetGameMode`))
    (:`then`
      (`/Game/Project/Blueprints/UI/PlayerUI.AbilityTuto` (`/Game/Project/Blueprints/Character/Proto3GameMode.PlayerUI` _asproto_3game_mode)))
    (:`CastFailed`
      _))
  (`self.SetInteracted` true)
  (bind (_direction _newtrack_0) (`Timeline|Timeline_0` :!via `PlayFromStart` :!label _label)
    (:`Update`
      (if (`self.IsPlayerNearby`)
        (`SceneComponent.K2_SetWorldRotation` (`self.SkeletalMesh`) (`KismetMathLibrary.RLerp` (`SceneComponent.K2_GetComponentRotation` _skeletalmesh) (`KismetMathLibrary.FindLookAtRotation` (`self.K2_GetActorLocation` (`GameplayStatics.GetPlayerPawn` 0)) (`SceneComponent.K2_GetComponentLocation` _skeletalmesh)) _newtrack_0 true) false false)
        (else
          (goto _label :!via `Stop`))))
    (:`Finished`
      (set `self.lookAtTaki` true)
      (`KismetSystemLibrary.PrintString` "End Start"))))

(event `self.Sphere.OnComponentEndOverlap`
  (params (OverlappedComponent :type "PrimitiveComponent Object Reference") (OtherActor :type "Actor Object Reference") (OtherComp :type "PrimitiveComponent Object Reference") (OtherBodyIndex :type Integer))
  (bind _skeletalmesh (`self.SkeletalMesh`))
  (bind _astaki (cast `/Game/Project/Blueprints/Character/Taki` OtherActor))
  (`/Game/Project/Blueprints/Character/PlayableCharacter.SetUIAbilityState` _astaki false)
  (set `/Game/Project/Blueprints/Character/Taki.CurrentPoiningMapCreature` null _astaki)
  (`KismetSystemLibrary.PrintString` "setting current map creature to null")
  (`self.SetInteracted` false)
  (set `self.lookAtTaki` false)
  (bind (_direction _newtrack_0) (`Timeline|Timeline` :!via `PlayFromStart` :!label _label_2)
    (:`Update`
      (if (`self.IsPlayerNearby`)
        (goto _label_2 :!via `Stop`)
        (else
          (`SceneComponent.K2_SetRelativeRotation` _skeletalmesh (`KismetMathLibrary.RLerp` (`SceneComponent.RelativeRotation` _skeletalmesh) (struct :`Yaw` 180.0) _newtrack_0 true) false false))))))

(event `SetInteracted`
  (params (NewState :type Boolean))
  (bind _outlinematerialinstance (`self.OutlineMaterialInstance`))
  (bind _output_get (set `self.IsPlayerNearby` NewState))
  (if _output_get
    (`MaterialInstanceDynamic.SetScalarParameterValue` _outlinematerialinstance "Thickness" 5.0)
    (else
      (`MaterialInstanceDynamic.SetScalarParameterValue` _outlinematerialinstance "Thickness" 0.0))))

(event `self.ReceiveTick`
  (params (DeltaSeconds :type "Float (single-precision)"))
  (`self.CalculateSpeed`)
  (bind _output_get (set `self.SplinePosition` (+ (* DeltaSeconds (`self.Speed`)) (`self.SplinePosition`))))
  (bind (_returnvalue_location _returnvalue_rotation) (`KismetMathLibrary.BreakTransform` (`SplineComponent.GetTransformAtDistanceAlongSpline` (`self.MovementRoute`) _output_get "Local" false)))
  (`SceneComponent.K2_SetRelativeLocationAndRotation` (`self.CharacterOffset`) _returnvalue_location _returnvalue_rotation false false)
  (if (>= (`self.SplinePosition`) (`SplineComponent.GetSplineLength` (`self.MovementRoute`)))
    (set `self.SplinePosition` 0.0)
    (`KismetSystemLibrary.PrintString` "Reseting splinepos"))
  (if (`self.lookAtTaki`)
    (`SceneComponent.K2_SetWorldRotation` (`self.SkeletalMesh`) (`KismetMathLibrary.FindLookAtRotation` (`self.K2_GetActorLocation` (`GameplayStatics.GetPlayerPawn` 0)) (`SceneComponent.K2_GetComponentLocation` (`self.SkeletalMesh`))) false false)
    (`KismetSystemLibrary.PrintString` "I am looking at Taki")))

(event `CalculateSpeed`
  (bind _niagara (`self.Niagara`))
  (if (`self.IsPlayerNearby`)
    (bind _output_get (set `self.Speed` (- (`self.Speed`) (* (`GameplayStatics.GetWorldDeltaSeconds`) (`self.Deceleration`)))))
    (if (< _output_get 0.0)
      (set `self.Speed` 0.0))
    (else
      (set `self.Speed` (+ (`self.Speed`) (* (`GameplayStatics.GetWorldDeltaSeconds`) (`self.Acceleration`))))
      (if (< (`self.MaxSpeed`) (`self.Speed`))
        (set `self.Speed` (`self.MaxSpeed`)))))
  (if (< (`self.Speed`) (`self.ParticlesThreshold`))
    (`ActorComponent.Deactivate` _niagara)
    (else
      (`ActorComponent.Activate` _niagara false))))

(fn `UserConstructionScript`)