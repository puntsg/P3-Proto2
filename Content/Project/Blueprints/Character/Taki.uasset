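; Taki is a player character Blueprint that can transform by swapping control to another creature.
; On IA_Transform it finds the first existing actor of the CreatureToSwap class, activates it, teleports it to Taki's transform and has player controller 0 possess it.
; It then deactivates itself and tells the Proto3GameMode's PlayerUI to update the transformation UI.
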(event `EnhancedInput|/Game/ThirdPerson/Input/Actions/IA_Transform`
  (params (ActionValue :type Boolean) (ElapsedSeconds :type "Float (double-precision)") (TriggeredSeconds :type "Float (double-precision)") (InputAction :type "InputAction Object Reference" :default "/Game/ThirdPerson/Input/Actions/IA_Transform.IA_Transform"))
  (:`Started`
    (bind _outactors (`GameplayStatics.GetAllActorsOfClass` (`self.CreatureToSwap`)))
    (bind _output (`|GetArrayItem` _outactors))
    (`/Engine/EditorBlueprintResources/StandardMacros.IsValid` _output
      (:`Is Valid`
        (bind _asplayable_character (cast `/Game/Project/Blueprints/Character/PlayableCharacter` _output))
        (`self.SetActive` _asplayable_character true)
        (`self.K2_SetActorTransform` _output (`self.GetTransform`) false true)
        (`Controller.Possess` (`GameplayStatics.GetPlayerController` 0) _output)
        (`self.SetActive` false)
        (bind _asproto_3game_mode (cast `/Game/Project/Blueprints/Character/Proto3GameMode` (`GameplayStatics.GetGameMode`)))
        (`/Game/Project/Blueprints/UI/PlayerUI.SetTransformationUI` (`/Game/Project/Blueprints/Character/Proto3GameMode.PlayerUI` _asproto_3game_mode))))))

(fn `UserConstructionScript`
  (`parent.UserConstructionScript`))