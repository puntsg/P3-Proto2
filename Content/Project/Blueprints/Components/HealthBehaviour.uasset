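; Health component that tracks an owner's current health, starting at MaxHealth on BeginPlay.
; Damage, Heal, MaxHeal and InstaKill change the value and fire event dispatchers for health change, hurt, heal and death.
; Heal fires the change event before clamping to MaxHealth, so listeners can see overheal.
; InstaKill fires only the death event, and Damage can leave Health below zero.
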(event `self.ReceiveBeginPlay`
  (set `self.Health` (`self.MaxHealth`)))

(fn `Damage`
  (params (Damage :type Integer))
  (bind _output_get (set `self.Health` (- (`self.Health`) Damage)))
  (`self.OnAlterHealth`)
  (if (<= _output_get 0)
    (`self.OnDie`)
    (else
      (`self.OnHurt`))))

(fn `Heal`
  (params (HealAmount :type Integer))
  (bind _maxhealth (`self.MaxHealth`))
  (bind _output_get (set `self.Health` (+ HealAmount (`self.Health`))))
  (`self.OnAlterHealth`)
  (if (> _output_get _maxhealth)
    (set `self.Health` _maxhealth))
  (`self.OnHeal`))

(fn `InstaKill`
  (set `self.Health` 0)
  (`self.OnDie`))

(fn `MaxHeal`
  (set `self.Health` (`self.MaxHealth`))
  (`self.OnAlterHealth`)
  (`self.OnHeal`))